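; Dream level component that makes itself levitate by bobbing up and down along its relative Z axis.
; BeginPlay picks a random phase offset and an amplitude within a configurable range, so instances move out of sync.
; Each Tick adds a sine of game time, scaled by Speed and amplitude, to the current relative location, so the motion accumulates per frame and depends on frame rate.
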(event `self.ReceiveBeginPlay`
  (set `self.Random Offset` (`KismetMathLibrary.RandomFloatInRange` 0.0 (* (`KismetMathLibrary.GetPI`) 2.0)))
  (set `self.Amplitude` (`KismetMathLibrary.RandomFloatInRange` (`self.Amplitude Min`) (`self.Amplitude Max`))))

(event `self.ReceiveTick`
  (params (DeltaSeconds :type "Float (single-precision)"))
  (`self.K2_SetRelativeLocation` self (+ (`self.RelativeLocation`) (`KismetMathLibrary.MakeVector` 0.0 0.0 (* (`KismetMathLibrary.Sin` (* (+ (`KismetSystemLibrary.GetGameTimeInSeconds`) (`self.Random Offset`)) (`self.Speed`))) (`self.Amplitude`)))) false false))