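; BP_Orb is a lobby decoration actor that pairs a colored magic orb effect with a configurable chain.
; The construction script adds ChainCount scaled-down static mesh links along Z, spaced by ChainLength from StartOffset.
; Within that same loop it passes OrbColor to the NSMagicOrb01 effect's FlareColor variable, so the color applies only when ChainCount is above zero.
; The event graph has no active runtime logic.
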(fn `UserConstructionScript`
  (for _index (range (`self.ChainCount`))
    (`AddComponent|NODE_AddStaticMeshComponent-0` :`RelativeTransform` (`KismetMathLibrary.MakeTransform` (`KismetMathLibrary.MakeVector` 0.0 0.0 (+ (`self.StartOffset`) (* _index (`self.ChainLength`)))) (struct) (0.2 0.2 0.2)))
    (`NiagaraComponent.SetVariableLinearColor` (`self.NS_MagicOrb01`) "FlareColor" (`self.OrbColor`))))