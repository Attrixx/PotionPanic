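; BP_Cauldron is the item visual for a cauldron, with a colored effect that reflects the item's gameplay tags.
; When tags change, the effect shows only if there is more than one tag, in a color derived from the tag container.
; SetEffectEnabled toggles the effect root and its children and tints the point light and sphere material.
; The construction script applies the default state and color.
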(event `self.OnItemTagsChanged`
  (params (NewTags :type "GameplayTagContainer Structure (by ref)"))
  (`self.SetEffectEnabled` (> (`BlueprintGameplayTagLibrary.GetNumGameplayTagsInContainer` NewTags) 1) (`CoreGameplayLibrary.MakeColorFromTagContainer` NewTags)))

(fn `SetEffectEnabled`
  (params (`Enabled?` :type Boolean :default true) (Color :type "LinearColor Structure" :default (struct :`R` 0.105995 :`G` 1.0 :`B` 0.468872 :`A` 1.0)))
  (`SceneComponent.SetVisibility` (`self.FullEffectRoot`) (`local.Enabled?`) true)
  (`LightComponent.SetLightColor` (`self.PointLight`) (`local.Color`) true)
  (`MeshComponent.SetColorParameterValueOnMaterials` (`self.Sphere`) "BaseColorFactor" (`local.Color`)))

(fn `UserConstructionScript`
  (`parent.UserConstructionScript`)
  (`self.SetEffectEnabled` (`self.EnabledByDefault`) (`self.DefaultColor`)))