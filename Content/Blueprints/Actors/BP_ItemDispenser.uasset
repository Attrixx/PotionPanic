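; BP_ItemDispenser is an interactable actor that hands a new item to an alchemist who is not already carrying one.
; On Interact, it casts the instigator to AlchemistBase and checks that its HolderComponent has no valid carriable.
; It then spawns an ItemClass actor at the holder's transform, assigns ItemAsset to it, and has the holder try to pick it up.
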(event `self.Interact`
  (params (Instigator :type "Actor Object Reference"))
  (bind _asalchemist_base (cast `AlchemistBase` Instigator))
  (bind _holdercomponent (`AlchemistBase.HolderComponent` _asalchemist_base))
  (`/Engine/EditorBlueprintResources/StandardMacros.IsValid` (`HolderComponent.GetCarriable` _holdercomponent)
    (:`Is Not Valid`
      (bind _returnvalue (`|SpawnActorFromClass` (`self.ItemClass`) (`SceneComponent.K2_GetComponentToWorld` _holdercomponent) "Undefined" "MultiplyWithRoot" self null))
      (`ItemActor.SetItemAsset` _returnvalue (`self.ItemAsset`))
      (`HolderComponent.TryPickup` _holdercomponent _returnvalue))))

(fn `UserConstructionScript`)