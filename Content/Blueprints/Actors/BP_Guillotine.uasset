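; BP_Guillotine is an animated guillotine actor whose blade moves up and down along with its rope.
; On BeginPlay, a timeline drives both the blade's relative height and the rope's vertical scale from one track, so the rope stretches as the blade lowers.
; When the timeline finishes, it restarts as long as the PlayAnimation flag is set, looping the motion.
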(event `self.ReceiveBeginPlay`
  (`self.PlayAnimation`))

(event `PlayAnimation`
  (bind (_direction _newtrack_0) (`Timeline|Timeline` :!via `PlayFromStart` :!label _label)
    (:`Update`
      (`SceneComponent.SetWorldScale3D` (`self.Rope`) (`KismetMathLibrary.MakeVector` 1.0 1.0 (`KismetMathLibrary.Lerp` 0.0 1.3 _newtrack_0)))
      (`SceneComponent.K2_SetRelativeLocation` (`self.SM_PROP_guillotine_blade`) (`KismetMathLibrary.MakeVector` 0.0 0.0 (`KismetMathLibrary.Lerp` 200.0 85.0 _newtrack_0)) false false))
    (:`Finished`
      (if (`self.bPlayAnimation`)
        (goto _label :!via `PlayFromStart`)))))

(fn `UserConstructionScript`)